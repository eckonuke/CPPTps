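; BP_OnlyEnemyManager is a timed spawner that creates BP_OnlyEnemy actors around the level's BP_SpawnPos points.
; BeginPlay gathers all spawn points, and Tick accumulates time against a random interval that is rerolled after each spawn.
; Spawn points are used round-robin through a modulo index.
; Each spawn first turns its point to a random yaw, then places the enemy a random distance along that forward vector.
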(event `self.ReceiveBeginPlay`
  ;[1 1 1] 초기생성시간 설정
  (set `self.createTime` (`KismetMathLibrary.RandomFloatInRange` (`self.randMin`) (`self.randMax`)))
  (bind _outactors (`GameplayStatics.GetAllActorsOfClass` "/Game/Blueprints/BP_SpawnPos.BP_SpawnPos_C"))
  (set `self.spawnPosArray` _outactors))

(event `self.ReceiveTick`
  (params (DeltaSeconds :type "Float (single-precision)"))
  (bind _output (`|GetArrayItem` (`self.spawnPosArray`) (mod (`self.spawnIndex`) (`KismetArrayLibrary.Array_Length` (`self.spawnPosArray`)))))
  (bind (_returnvalue_location _returnvalue_rotation _returnvalue_scale) (`KismetMathLibrary.BreakTransform` (`self.GetTransform` _output)))
  ;[1 1 1] 시간을 흐르게 한다
  (bind _output_get (set `self.currTime` (+ DeltaSeconds (`self.currTime`))))
  ;[1 1 1] 만약 생성시간이 되었다면
  (if (> _output_get (`self.createTime`))
    ;[1 1 1] 에너미가 나가야할 방향을 정한다
    (`self.K2_SetActorRotation` _output (`KismetMathLibrary.MakeRotator` 0.0 0.0 (`KismetMathLibrary.RandomFloatInRange` 0.0 359.0)) false)
    ;[1 1 1] Enemy생성 해서 내 위치에 놓는다
    (`|SpawnActorFromClass` "/Game/Blueprints/OnlyBlueprint/BP_OnlyEnemy.BP_OnlyEnemy_C" (`KismetMathLibrary.MakeTransform` (+ (* (`self.GetActorForwardVector` _output) (`KismetMathLibrary.RandomFloatInRange` 100.0 500.0)) _returnvalue_location) _returnvalue_rotation _returnvalue_scale) "Undefined" "OverrideRootScale" null null)
    ;[1 1 1] 초기화
    (set `self.currTime` 0.0)
    (set `self.createTime` (`KismetMathLibrary.RandomFloatInRange` (`self.randMin`) (`self.randMax`)))
    ;[1 1 1] 다음순서로 넘어간다
    (`/Engine/EditorBlueprintResources/StandardMacros.IncrementInt` (`self.spawnIndex`))))

(fn `UserConstructionScript`)