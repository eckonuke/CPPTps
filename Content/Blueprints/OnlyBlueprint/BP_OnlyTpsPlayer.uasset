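; Third-person shooter player character with walk/run, jump, camera look and switching between rifle and sniper, starting on sniper.
; InputFire plays the ABP_OnlyPlayer attack, then branches on rifle visibility: rifle spawns BP_OnlyBullet, sniper line-traces from the camera.
; Sniper hits spawn an explosion, push physics bodies with mass-scaled force, or call ReceiveDamage on a BP_OnlyEnemy's FSM.
; Zoom narrows FOV and swaps common and sniper widgets, whichever weapon is shown.
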(event `InputAxis|Vertical`
  (params (AxisValue :type "Float (single-precision)"))
  (bind (_returnvalue_roll _returnvalue_pitch _returnvalue_yaw) (`KismetMathLibrary.BreakRotator` (`self.GetControlRotation`)))
  ;[1 1 1] 플레이어 움직임
  (`self.AddMovementInput` (`KismetMathLibrary.GetForwardVector` (`KismetMathLibrary.MakeRotator` 0.0 0.0 _returnvalue_yaw)) AxisValue))

(event `InputAction|Run`
  (params (Key :type "Key Structure"))
  (bind _charactermovement (`self.CharacterMovement`))
  ;[1 1 1] Character Run
  (:`Pressed`
    (set `CharacterMovementComponent.MaxWalkSpeed` (`self.runSpeed`) _charactermovement))
  (:`Released`
    (set `CharacterMovementComponent.MaxWalkSpeed` (`self.walkSpeed`) _charactermovement)))

(event `InputAxis|Horizontal`
  (params (AxisValue :type "Float (single-precision)"))
  (bind (_returnvalue_roll _returnvalue_pitch _returnvalue_yaw) (`KismetMathLibrary.BreakRotator` (`self.GetControlRotation`)))
  ;[1 1 1] 플레이어 움직임
  (`self.AddMovementInput` (`KismetMathLibrary.GetRightVector` (`KismetMathLibrary.MakeRotator` _returnvalue_roll 0.0 _returnvalue_yaw)) AxisValue))

(event `InputAxis|Turn`
  (params (AxisValue :type "Float (single-precision)"))
  ;[1 1 1] 카메라 회전
  (`self.AddControllerYawInput` AxisValue))

(event `InputAction|Jump`
  (params (Key :type "Key Structure"))
  ;[1 1 1] 점프
  (:`Pressed`
    (`self.Jump`))
  (:`Released`
    (`self.StopJumping`)))

(event `InputAxis|LookUp`
  (params (AxisValue :type "Float (single-precision)"))
  ;[1 1 1] 카메라 회전
  (`self.AddControllerPitchInput` AxisValue))

(event `InputAction|Rifle`
  (params (Key :type "Key Structure"))
  ;[1 1 1] Show Rifle
  (:`Pressed`
    (`self.ChangeWeapon` false)))

(event `InputAction|Fire`
  (params (Key :type "Key Structure"))
  ;[1 1 1] Fire
  (:`Pressed`
    (`self.InputFire`)))

(event `InputAction|Sniper`
  (params (Key :type "Key Structure"))
  ;[1 1 1] Show Sniper
  (:`Pressed`
    (`self.ChangeWeapon` true)))

(event `InputAction|Zoom`
  (params (Key :type "Key Structure"))
  (bind _commonui (`self.CommonUI`))
  (bind _sniperui (`self.SniperUI`))
  (bind _camera (`self.Camera`))
  ;[1 1 1] Zoom
  (:`Pressed`
    (`UserWidget.AddToViewport` _sniperui 0)
    (`CameraComponent.SetFieldOfView` _camera 30.0)
    (`Widget.RemoveFromParent` _commonui))
  (:`Released`
    (`Widget.RemoveFromParent` _sniperui)
    (`CameraComponent.SetFieldOfView` _camera 90.0)
    (`UserWidget.AddToViewport` _commonui 0)))

(event `self.ReceiveBeginPlay`
  (`self.ChangeWeapon` true)
  (bind _returnvalue (`|CreateWidget` "/Game/Blueprints/SniperUI.SniperUI_C"))
  (set `self.SniperUI` _returnvalue)
  (bind _returnvalue_2 (`|CreateWidget` "/Game/Blueprints/CommonUI.CommonUI_C"))
  (bind _output_get (set `self.CommonUI` _returnvalue_2))
  (`UserWidget.AddToViewport` _output_get 0))

(fn `ChangeWeapon`
  (params (useSniper :type Boolean))
  (`SceneComponent.SetVisibility` (`self.Sniper`) useSniper false)
  (`SceneComponent.SetVisibility` (`self.Gun`) (not useSniper) false))

(fn `InputFire`
  (bind _camera (`self.Camera`))
  (bind _returnvalue (`SceneComponent.K2_GetComponentLocation` _camera))
  (bind _asabp_only_player (cast `/Game/Blueprints/OnlyBlueprint/ABP_OnlyPlayer` (`SkeletalMeshComponent.GetAnimInstance` (`self.Mesh`))))
  (`/Game/Blueprints/OnlyBlueprint/ABP_OnlyPlayer.PlayAttackAnim` _asabp_only_player)
  ;[1 1 1] 라이플 총이 보이냐
  (if (`SceneComponent.bVisible` (`self.Gun`))
    ;[1 1 1] 라이플 총알 발사
    (`|SpawnActorFromClass` "/Game/Blueprints/OnlyBlueprint/BP_OnlyBullet.BP_OnlyBullet_C" (`SceneComponent.GetSocketTransform` (`self.Gun`) "FirePos" "RTS_World") "Undefined" "OverrideRootScale" null null)
    (else
      (bind (_outhit _returnvalue_2) (`KismetSystemLibrary.LineTraceSingle` :`Start` _returnvalue :`End` (+ _returnvalue (* (`SceneComponent.GetForwardVector` _camera) 5000.0)) :`TraceChannel` "TraceTypeQuery1" :`DrawDebugType` "ForDuration"))
      (if _returnvalue_2
        (bind (_bblockinghit _binitialoverlap _time _distance _location _impactpoint _normal _impactnormal _physmat _hitactor _hitcomponent) (`GameplayStatics.BreakHitResult` _outhit))
        (`GameplayStatics.SpawnEmitterAtLocation` "/Game/StarterContent/Particles/P_Explosion.P_Explosion" _impactpoint)
        (if (`SceneComponent.IsSimulatingPhysics` _hitcomponent "None")
          (`PrimitiveComponent.AddForceAtLocation` _hitcomponent (* (`SceneComponent.GetForwardVector` (`self.Camera`)) 100000.0 (`PrimitiveComponent.GetMass` _hitcomponent)) _impactpoint "None")
          (else
            ;[1 1 1] 만약에 맞은놈이 Enemy라면 ReceiveDamage 함수를 호출
            (bind _asbp_only_enemy (cast `/Game/Blueprints/OnlyBlueprint/BP_OnlyEnemy` _hitactor))
            (`/Game/Blueprints/OnlyBlueprint/BP_OnlyEnemyFSM.receiveDamage` (`/Game/Blueprints/OnlyBlueprint/BP_OnlyEnemy.FSM` _asbp_only_enemy))))))))

(fn `UserConstructionScript`)