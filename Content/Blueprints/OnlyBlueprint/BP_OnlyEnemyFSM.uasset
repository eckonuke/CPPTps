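; Enemy AI component that runs BP_OnlyEnemy as a Tick-driven state machine targeting BP_OnlyTpsPlayer.
; Idle spots the player with a view-cone check and line trace, Move chases into range, and Attack only prints before a timed delay.
; ReceiveDamage decrements health into a timed Damaged stagger or Die, which disables capsule collision and sinks the enemy until destroyed.
; ChangeState mirrors each state to ABP_OnlyEnemy and plays the hit montage.
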(event `self.ReceiveBeginPlay`
  ;[1 1 1] Target 찾자(Player)
  (bind _returnvalue (`GameplayStatics.GetActorOfClass` "/Game/Blueprints/OnlyBlueprint/BP_OnlyTpsPlayer.BP_OnlyTpsPlayer_C"))
  (set `self.target` _returnvalue)
  ;[1 1 1] 나를 찾자
  (bind _asbp_only_enemy (cast `/Game/Blueprints/OnlyBlueprint/BP_OnlyEnemy` (`self.GetOwner`)))
  (set `self.me` _asbp_only_enemy)
  ;[1 1 1] 초기 HP 설정
  (set `self.currHealth` (`self.maxHealth`))
  ;[1 1 1] Animation Blueprint 가져오기
  (bind _asabp_only_enemy (cast `/Game/Blueprints/OnlyBlueprint/ABP_OnlyEnemy` (`SkeletalMeshComponent.GetAnimInstance` (`Character.Mesh` (`self.me`)))))
  (set `self.anim` _asabp_only_enemy))

(event `self.ReceiveTick`
  (params (DeltaSeconds :type "Float (single-precision)"))
  (switch `/Game/Blueprints/OnlyBlueprint/BP_EnemyState` (`self.state`)
    (:`NewEnumerator0`
      (`self.Update Idle`))
    (:`NewEnumerator1`
      (`self.UpdateMove`))
    (:`NewEnumerator2`
      (`self.UpdateAttack`))
    (:`NewEnumerator3`
      (`self.UpdateDamaged`))
    (:`NewEnumerator4`
      (`self.UpdateDie`))
    (:`NewEnumerator5`
      (`self.UpdateAttackDelay`))))

(fn `changeState`
  (params (oldState :type "/Game/Blueprints/OnlyBlueprint/BP_EnemyState Enum" :default "NewEnumerator0"))
  (bind _output_get (set `self.state` oldState))
  (bind _output_get_2 (set `/Game/Blueprints/OnlyBlueprint/ABP_OnlyEnemy.state` _output_get (`self.anim`)))
  (switch `/Game/Blueprints/OnlyBlueprint/BP_EnemyState` _output_get_2
    (:`NewEnumerator3`
      (`Character.PlayAnimMontage` (`self.me`) "/Game/Blueprints/AMT_EnemyDamage.AMT_EnemyDamage" 1.0 "None"))
    (:`NewEnumerator4`
      (`PrimitiveComponent.SetCollisionEnabled` (`Character.CapsuleComponent` (`self.me`)) "NoCollision"))))

(fn `receiveDamage`
  (bind _output_get (set `self.currHealth` (- (`self.currHealth`) 1.0)))
  (if (> _output_get 0.0)
    (`self.changeState` "NewEnumerator3")
    (else
      (`self.changeState` "NewEnumerator4"))))

(fn `Update Idle`
  ;[1 1 1] 만약에 두 벡터 사이의 각이 30보다 작으면 (시야60)
  (if (< (`KismetMathLibrary.DegAcos` (`KismetMathLibrary.Dot_VectorVector` (`Actor.GetActorForwardVector` (`self.me`)) (`KismetMathLibrary.Normal` (- (`Actor.K2_GetActorLocation` (`self.target`)) (`Actor.K2_GetActorLocation` (`self.me`)))))) 30.0)
    (bind _outhit (`KismetSystemLibrary.LineTraceSingle` (`Actor.K2_GetActorLocation` (`self.me`)) (`Actor.K2_GetActorLocation` (`self.target`)) "TraceTypeQuery1"))
    (if (`KismetStringLibrary.Contains` (`KismetSystemLibrary.GetDisplayName` (`.HitActor` (`GameplayStatics.BreakHitResult` _outhit))) "Player")
      (`self.changeState` "NewEnumerator1"))))

(fn `UpdateAttack`
  (`KismetSystemLibrary.PrintString` "Attack!!!!!!!!!!!!")
  (`self.changeState` "NewEnumerator5"))

(fn `UpdateAttackDelay`
  (bind _bcomplete (`self.UpdateTime` (`self.attackDelayTime`)))
  (if _bcomplete
    (if (< (`KismetMathLibrary.VSize` (- (`Actor.K2_GetActorLocation` (`self.target`)) (`Actor.K2_GetActorLocation` (`self.me`)))) (`self.attackRange`))
      (`self.changeState` "NewEnumerator2")
      (else
        (`self.changeState` "NewEnumerator0")))))

(fn `UpdateDamaged`
  (bind _bcomplete (`self.UpdateTime` (`self.damageDelayTime`)))
  (if _bcomplete
    (`self.changeState` "NewEnumerator1")))

(fn `UpdateDie`
  (bind _me (`self.me`))
  (bind (_returnvalue_x _returnvalue_y _returnvalue_z) (`KismetMathLibrary.BreakVector` (`Actor.K2_GetActorLocation` (`self.me`))))
  (`Actor.K2_SetActorLocation` _me (+ (`Actor.K2_GetActorLocation` _me) (* (`self.dieSpeed`) (`KismetMathLibrary.Vector_Down`) (`GameplayStatics.GetWorldDeltaSeconds`))) false false)
  (if (< _returnvalue_z -200.0)
    (`Actor.K2_DestroyActor` (`self.me`))))

(fn `UpdateMove`
  (bind _returnvalue (- (`Actor.K2_GetActorLocation` (`self.target`)) (`Actor.K2_GetActorLocation` (`self.me`))))
  ;[1 1 1] 만약에 공격범위에 target이 들어왔다면 상태를 Attack으로
  (if (< (`KismetMathLibrary.VSize` _returnvalue) (`self.attackRange`))
    (`self.changeState` "NewEnumerator2")
    (else
      (`Pawn.AddMovementInput` (`self.me`) (`KismetMathLibrary.Normal` _returnvalue) 1.0 false))))

(fn `UpdateTime`
  (params (delayTime :type "Float (double-precision)"))
  (returns (bComplete :type Boolean))
  (bind _output_get (set `self.currentTime` (+ (`GameplayStatics.GetWorldDeltaSeconds`) (`self.currentTime`))))
  (if (== (> _output_get delayTime) true)
    (set `self.currentTime` 0.0)
    (return true)
    (else
      (return false))))